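; Game manager for a find-the-molecule level: picks a random target compound, shows its sprite and runs win/lose logic.
; Tick calls Spawn until one target and five of each other compound are randomly placed within a box.
; After a startup delay, Tick infers clicks from changes in the "Clickable" actor count.
; A missing target pauses with SuccessUI; other removals advance the GameUI health/angel meter, eventually pausing with GameOverUI.
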(event EventTick
  (params (DeltaSeconds :type Float%20%28single-precision%29))
  (bind _spritelist (Variables|Default|GetSpriteList))
  ;[1 1 1] Sets the "chosen" compound and spawns all compunds
  (Utilities|FlowControl|Sequence
    (:then_0
      (Utilities|FlowControl|DoOnce false
        (:Completed
          (bind _output_get (Variables|Default|SetEnum (Utilities|Select :Index (Math|Random|RandomIntegerinRange 0 7) :Option%200 "NewEnumerator0" :Option%201 "NewEnumerator1" :Option%202 "NewEnumerator2" :Option%203 "NewEnumerator3" :Option%204 "NewEnumerator4" :Option%205 "NewEnumerator5" :Option%206 "NewEnumerator6" :Option%207 "NewEnumerator7"))))))
    (:then_1
      (CallFunction|Spawn _output_get)
      ;[1 1 1] Sets the Find: sprite to the chosen compound
      (Rendering|Components|Sprite|SetSprite (Variables|Default|GetPaperSprite) (Utilities|Select :Index (Variables|Default|GetEnum) :NewEnumerator0 (.h2o _spritelist) :NewEnumerator1 (.co2 _spritelist) :NewEnumerator2 (.h2o2 _spritelist) :NewEnumerator3 (.o2 _spritelist) :NewEnumerator4 (.nh3 _spritelist) :NewEnumerator5 (.ch20 _spritelist) :NewEnumerator6 (.ch30h _spritelist) :NewEnumerator7 (.ch4 _spritelist)))
      ;[1 1 1] Check If A Molecule Has Been Clicked On
      (if (== (Variables|Default|GetDelayCompleted) true)
        (bind _outactors (Actor|GetAllActorswithTag "Clickable"))
        (Variables|Default|SetCurrentMolecules (Utilities|Array|Length _outactors))
        ;[1 1 1] Check If Right Molecule Has Been Clicked On
        (if (!= (Variables|Default|GetCurrentMolecules) (Variables|Default|GetTotalMolecules))
          (bind _outactors_2 (Actor|GetAllActorsOfClass (Utilities|Select :Index (Variables|Default|GetEnum) :NewEnumerator0 "/Game/Blueprints/Molecules/H20.H20_C" :NewEnumerator1 "/Game/Blueprints/Molecules/CO2.CO2_C" :NewEnumerator2 "/Game/Blueprints/Molecules/H2O2.H2O2_C" :NewEnumerator3 "/Game/Blueprints/Molecules/O2.O2_C" :NewEnumerator4 "/Game/Blueprints/Molecules/NH3.NH3_C" :NewEnumerator5 "/Game/Blueprints/Molecules/CH20.CH20_C" :NewEnumerator6 "/Game/Blueprints/Molecules/CH30H.CH30H_C" :NewEnumerator7 "/Game/Blueprints/Molecules/CH4.CH4_C")))
          (if (< (Utilities|Array|Length _outactors_2) 1)
            ;[1 1 1] Level Complete Screen
            (Game|SetGamePaused true)
            (Audio|PlaySound2D "/Game/Sounds/winSound.winSound" 1.0 1.0 0.0 0 0)
            (bind _returnvalue (UserInterface|CreateWidget "/Game/Blueprints/SuccessUI.SuccessUI_C"))
            (UserInterface|Viewport|AddtoViewport _returnvalue 0)
            (else
              ;[1 1 1] If Wrong Deduct Health
              (if (< (Class|Slider|GetValue (Variables|/Game/Blueprints/GameUI.GameUI_C|GetHealth (Variables|Default|GetProgressBar))) 2.7)
                (Default|UpdateAngel (Variables|Default|GetProgressBar) (+ (Class|Slider|GetValue (Variables|/Game/Blueprints/GameUI.GameUI_C|GetHealth (Variables|Default|GetProgressBar))) 0.95))
                (Variables|Default|SetTotalMolecules (Variables|Default|GetCurrentMolecules))
                (Audio|PlaySound2D "/Game/Sounds/weepingAngelsMoving.weepingAngelsMoving" 1.0 1.0 0.0 0 0)
                (else
                  ;[1 1 1] Game Over Screen
                  (Default|UpdateAngel (Variables|Default|GetProgressBar) (+ (Class|Slider|GetValue (Variables|/Game/Blueprints/GameUI.GameUI_C|GetHealth (Variables|Default|GetProgressBar))) 0.9))
                  (Game|SetGamePaused true)
                  (Audio|PlaySound2D "/Game/Sounds/loseSound.loseSound" 1.0 1.0 0.0 0 0)
                  (bind _returnvalue_2 (UserInterface|CreateWidget "/Game/Blueprints/GameOverUI.GameOverUI_C"))
                  (UserInterface|Viewport|AddtoViewport _returnvalue_2 0))))))
        (else
          (Utilities|FlowControl|Delay 2.0)
          (Variables|Default|SetDelayCompleted true))))))

(event EventBeginPlay
  (Utilities|FlowControl|Sequence
    (:then_0
      ;[1 1 1] Create HUD
      (bind _returnvalue (UserInterface|CreateWidget "/Game/Blueprints/GameUI.GameUI_C"))
      (bind _output_get (Variables|Default|SetProgressBar _returnvalue))
      (UserInterface|Viewport|AddtoViewport _output_get 0))
    (:then_1
      ;[1 1 1] Get Total Molecules
      (Utilities|FlowControl|Delay 1.0)
      (bind _outactors (Actor|GetAllActorswithTag "Clickable"))
      (bind _output_get_2 (Variables|Default|SetTotalMolecules (Utilities|Array|Length _outactors)))
      (Variables|Default|SetCurrentMolecules _output_get_2))))

(fn ConstructionScript)

(fn Spawn
  (params (Enum :type Enum%20Enum :default "NewEnumerator0"))
  (bind _returnvalue (Math|Random|RandomFloatinRange 0.0 3.6e+02))
  (bind _returnvalue_2 (Math|Random|RandomFloatinRange 0.0 3.6e+02))
  (bind _returnvalue_3 (Math|Random|RandomFloatinRange 0.0 3.6e+02))
  (bind _defaultsceneroot (Variables|Default|GetDefaultSceneRoot))
  (bind _returnvalue_4 (Transformation|GetWorldLocation _defaultsceneroot))
  (bind _returnvalue_5 (Math|Random|RandomPointinBoundingBox _returnvalue_4 "900.000000,0.000000,275.000000"))
  ;[1 1 1] Spawn Molecules At Random Location
  (Variables|Default|SetEnum Enum)
  (Utilities|FlowControl|Sequence
    (:then_0
      (if (not (>= (Variables|Default|GetO2%20Count) (Utilities|Select :Index (Variables|Default|Getenum) :NewEnumerator0 5 :NewEnumerator1 5 :NewEnumerator2 5 :NewEnumerator3 1 :NewEnumerator4 5 :NewEnumerator5 5 :NewEnumerator6 5 :NewEnumerator7 5)))
        (Game|SpawnActorfromClass "/Game/Blueprints/Molecules/O2.O2_C" (Math|Transform|MakeTransform _returnvalue_5 (Math|Rotator|MakeRotator 0.0 _returnvalue 0.0) "0.750000,0.750000,0.750000") "Undefined" 0 0)
        (Math|Integer|IncrementInt (Variables|Default|GetO2%20Count))))
    (:then_1
      (if (not (>= (Variables|Default|GetH2O%20Count) (Utilities|Select :Index (Variables|Default|Getenum) :NewEnumerator0 1 :NewEnumerator1 5 :NewEnumerator2 5 :NewEnumerator3 5 :NewEnumerator4 5 :NewEnumerator5 5 :NewEnumerator6 5 :NewEnumerator7 5)))
        (Game|SpawnActorfromClass "/Game/Blueprints/Molecules/H20.H20_C" (Math|Transform|MakeTransform _returnvalue_5 (Math|Rotator|MakeRotator 0.0 _returnvalue 0.0) "0.750000,0.750000,0.750000") "Undefined" 0 0)
        (Math|Integer|IncrementInt (Variables|Default|GetH2O%20Count))))
    (:then_2
      (if (not (>= (Variables|Default|GetH2O2%20Count) (Utilities|Select :Index (Variables|Default|Getenum) :NewEnumerator0 5 :NewEnumerator1 5 :NewEnumerator2 1 :NewEnumerator3 5 :NewEnumerator4 5 :NewEnumerator5 5 :NewEnumerator6 5 :NewEnumerator7 5)))
        (Game|SpawnActorfromClass "/Game/Blueprints/Molecules/H2O2.H2O2_C" (Math|Transform|MakeTransform _returnvalue_5 (Math|Rotator|MakeRotator 0.0 _returnvalue_3 0.0) "0.750000,0.750000,0.750000") "Undefined" 0 0)
        (Math|Integer|IncrementInt (Variables|Default|GetH2O2%20Count))))
    (:then_3
      (if (not (>= (Variables|Default|GetCO2%20Count) (Utilities|Select :Index (Variables|Default|Getenum) :NewEnumerator0 5 :NewEnumerator1 1 :NewEnumerator2 5 :NewEnumerator3 5 :NewEnumerator4 5 :NewEnumerator5 5 :NewEnumerator6 5 :NewEnumerator7 5)))
        (Game|SpawnActorfromClass "/Game/Blueprints/Molecules/CO2.CO2_C" (Math|Transform|MakeTransform _returnvalue_5 (Math|Rotator|MakeRotator 0.0 _returnvalue_3 0.0) "0.750000,0.750000,0.750000") "Undefined" 0 0)
        (Math|Integer|IncrementInt (Variables|Default|GetCO2%20Count))))
    (:then_4
      (if (not (>= (Variables|Default|GetNH3%20Count) (Utilities|Select :Index (Variables|Default|Getenum) :NewEnumerator0 5 :NewEnumerator1 5 :NewEnumerator2 5 :NewEnumerator3 5 :NewEnumerator4 1 :NewEnumerator5 5 :NewEnumerator6 5 :NewEnumerator7 5)))
        (Game|SpawnActorfromClass "/Game/Blueprints/Molecules/NH3.NH3_C" (Math|Transform|MakeTransform _returnvalue_5 (Math|Rotator|MakeRotator 0.0 _returnvalue_3 0.0) "0.750000,0.750000,0.750000") "Undefined" 0 0)
        (Math|Integer|IncrementInt (Variables|Default|GetNH3%20Count))))
    (:then_5
      (if (not (>= (Variables|Default|GetCH20%20Count) (Utilities|Select :Index (Variables|Default|Getenum) :NewEnumerator0 5 :NewEnumerator1 5 :NewEnumerator2 5 :NewEnumerator3 5 :NewEnumerator4 5 :NewEnumerator5 1 :NewEnumerator6 5 :NewEnumerator7 5)))
        (Game|SpawnActorfromClass "/Game/Blueprints/Molecules/CH20.CH20_C" (Math|Transform|MakeTransform _returnvalue_5 (Math|Rotator|MakeRotator 0.0 _returnvalue_2 0.0) "0.750000,0.750000,0.750000") "Undefined" 0 0)
        (Math|Integer|IncrementInt (Variables|Default|GetCH20%20Count))))
    (:then_6
      (if (not (>= (Variables|Default|GetCH30H%20Count) (Utilities|Select :Index (Variables|Default|Getenum) :NewEnumerator0 5 :NewEnumerator1 5 :NewEnumerator2 5 :NewEnumerator3 5 :NewEnumerator4 5 :NewEnumerator5 5 :NewEnumerator6 1 :NewEnumerator7 5)))
        (Game|SpawnActorfromClass "/Game/Blueprints/Molecules/CH30H.CH30H_C" (Math|Transform|MakeTransform _returnvalue_5 (Math|Rotator|MakeRotator 0.0 _returnvalue_2 0.0) "0.750000,0.750000,0.750000") "Undefined" 0 0)
        (Math|Integer|IncrementInt (Variables|Default|GetCH30H%20Count))))
    (:then_7
      (if (not (>= (Variables|Default|GetCH4%20Count) (Utilities|Select :Index (Variables|Default|Getenum) :NewEnumerator0 5 :NewEnumerator1 5 :NewEnumerator2 5 :NewEnumerator3 5 :NewEnumerator4 5 :NewEnumerator5 5 :NewEnumerator6 5 :NewEnumerator7 1)))
        (Game|SpawnActorfromClass "/Game/Blueprints/Molecules/CH4.CH4_C" (Math|Transform|MakeTransform _returnvalue_5 (Math|Rotator|MakeRotator 0.0 _returnvalue_2 0.0) "0.750000,0.750000,0.750000") "Undefined" 0 0)
        (Math|Integer|IncrementInt (Variables|Default|GetCH4%20Count))))))