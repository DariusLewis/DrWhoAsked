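; GameManager runs a molecule-clicking level in which H2O is the correct pick.
; After a startup delay it creates the HUD and counts the actors of five molecule classes.
; Tick polls the "Clickable" tag count to detect removed molecules: fewer H2O pauses the game with a success screen.
; Any other loss advances the HUD slider as a health penalty, pausing with game over once it passes its threshold.
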(event EventTick
  (params (DeltaSeconds :type Float%20%28single-precision%29))
  ;[1 1 1] Check If A Molecule Has Been Clicked On
  (if (== (Variables|Default|GetDelayCompleted) true)
    (bind _outactors (Actor|GetAllActorswithTag "Clickable"))
    (Variables|Default|SetCurrentMolecules (Utilities|Array|Length _outactors))
    (if (!= (Variables|Default|GetCurrentMolecules) (Variables|Default|GetTotalMolecules))
      ;[1 1 1] Check If Right Molecule Has Been Clicked On
      (bind _outactors_2 (Actor|GetAllActorsOfClass "/Game/Blueprints/H20.H20_C"))
      (Variables|Default|SetCurrentH2O (Utilities|Array|Length _outactors_2))
      (if (< (Variables|Default|GetCurrentH2O) (Variables|Default|GetTotalH20))
        ;[1 1 1] Level Complete Screen
        (Variables|Default|SetTotalMolecules (Variables|Default|GetCurrentMolecules))
        (Variables|Default|SetTotalH20 (Variables|Default|GetCurrentH2O))
        (Game|SetGamePaused true)
        (bind _returnvalue (UserInterface|CreateWidget "/Game/Blueprints/SuccessUI.SuccessUI_C"))
        (UserInterface|Viewport|AddtoViewport _returnvalue 0)
        (else
          ;[1 1 1] If Wrong Deduct Health
          (if (< (Class|Slider|GetValue (Variables|/Game/Blueprints/GameUI.GameUI_C|GetSlider_1 (Variables|Default|GetScoreUI))) 2.7)
            (Default|UpdateAngel (Variables|Default|GetScoreUI) (+ (Class|Slider|GetValue (Variables|/Game/Blueprints/GameUI.GameUI_C|GetSlider_1 (Variables|Default|GetScoreUI))) 0.95))
            (Variables|Default|SetTotalMolecules (Variables|Default|GetCurrentMolecules))
            (else
              ;[1 1 1] Game Over Screen
              (Default|UpdateAngel (Variables|Default|GetScoreUI) (+ (Class|Slider|GetValue (Variables|/Game/Blueprints/GameUI.GameUI_C|GetSlider_1 (Variables|Default|GetScoreUI))) 0.9))
              (Game|SetGamePaused true)
              (bind _returnvalue_2 (UserInterface|CreateWidget "/Game/Blueprints/GameOverUI.GameOverUI_C"))
              (UserInterface|Viewport|AddtoViewport _returnvalue_2 0))))))
    (else
      (Utilities|FlowControl|Delay 2.0)
      (Variables|Default|SetDelayCompleted true))))

(event EventBeginPlay
  (Utilities|FlowControl|Delay 1.5)
  (Utilities|FlowControl|Sequence
    (:then_0
      ;[1 1 1] Create HUD
      (bind _returnvalue (UserInterface|CreateWidget "/Game/Blueprints/GameUI.GameUI_C"))
      (bind _output_get (Variables|Default|SetScoreUI _returnvalue))
      (UserInterface|Viewport|AddtoViewport _output_get 0))
    (:then_1
      ;[1 1 1] Set Current And Total Molecule Values
      (bind _outactors (Actor|GetAllActorsOfClass "/Game/Blueprints/H2O2.H2O2_C"))
      (bind _output_get_2 (Variables|Default|SetTotalH2O2 (Utilities|Array|Length _outactors)))
      (bind _output_get_3 (Variables|Default|SetCurrentH2O2 _output_get_2))
      (bind _output_get_4 (Variables|Default|SetTotalMolecules (+ _output_get_3 (stale _output_get_6) (stale _output_get_8) (stale _output_get_10) (stale _output_get_12)) :!label _label))
      (Variables|Default|SetCurrentMolecules _output_get_4))
    (:then_2
      (bind _outactors_2 (Actor|GetAllActorsOfClass "/Game/Blueprints/H20.H20_C"))
      (bind _output_get_5 (Variables|Default|SetTotalH20 (Utilities|Array|Length _outactors_2)))
      (bind _output_get_6 (Variables|Default|SetCurrentH2O _output_get_5))
      (goto _label))
    (:then_3
      (bind _outactors_3 (Actor|GetAllActorsOfClass "/Game/Blueprints/O2.O2_C"))
      (bind _output_get_7 (Variables|Default|SetTotalO2 (Utilities|Array|Length _outactors_3)))
      (bind _output_get_8 (Variables|Default|SetCurrentO2 _output_get_7))
      (goto _label))
    (:then_4
      (bind _outactors_4 (Actor|GetAllActorsOfClass "/Game/Blueprints/CO2.CO2_C"))
      (bind _output_get_9 (Variables|Default|SetTotalCO2 (Utilities|Array|Length _outactors_4)))
      (bind _output_get_10 (Variables|Default|SetCurrentCO2 _output_get_9))
      (goto _label))
    (:then_5
      (bind _outactors_5 (Actor|GetAllActorsOfClass "/Game/Blueprints/NH3.NH3_C"))
      (bind _output_get_11 (Variables|Default|SetTotalNH3 (Utilities|Array|Length _outactors_5)))
      (bind _output_get_12 (Variables|Default|SetCurrentNH3 _output_get_11))
      (goto _label))))

(fn ConstructionScript)