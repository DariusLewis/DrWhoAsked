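; Spawner actor that fills the area around itself with molecule actors: O2, H2O, H2O2, CO2 and NH3.
; Each Tick, a sequence spawns up to one of each type at a random point in a flat X-Z box and increments that type's counter.
; H2O is capped at one, while the others compare against a random limit re-rolled every Tick.
; Counters are never decremented here.
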(event EventTick
  (params (DeltaSeconds :type Float%20%28single-precision%29))
  (bind _defaultsceneroot (Variables|Default|GetDefaultSceneRoot))
  (bind _returnvalue (Transformation|GetWorldLocation _defaultsceneroot))
  (bind _returnvalue_2 (Math|Random|RandomPointinBoundingBox _returnvalue "900.000000,0.000000,275.000000"))
  ;[1 1 1] Spawn Molecules At Random Location
  (Utilities|FlowControl|Sequence
    (:then_0
      (if (not (>= (Variables|Default|GetO2%20Count) (Math|Random|RandomIntegerinRange 10 15)))
        (Game|SpawnActorfromClass "/Game/Blueprints/O2.O2_C" (Math|Transform|MakeTransform _returnvalue_2 "0, 0, 0" "0.750000,0.750000,0.750000") "Undefined" 0 0)
        (Math|Integer|IncrementInt (Variables|Default|GetO2%20Count))))
    (:then_1
      (if (not (>= (Variables|Default|GetH2O%20Count) 1))
        (Game|SpawnActorfromClass "/Game/Blueprints/H20.H20_C" (Math|Transform|MakeTransform _returnvalue_2 "0, 0, 0" "0.750000,0.750000,0.750000") "Undefined" 0 0)
        (Math|Integer|IncrementInt (Variables|Default|GetH2O%20Count))))
    (:then_2
      (if (not (>= (Variables|Default|GetH2O2%20Count) (Math|Random|RandomIntegerinRange 10 15)))
        (Game|SpawnActorfromClass "/Game/Blueprints/H2O2.H2O2_C" (Math|Transform|MakeTransform _returnvalue_2 "0, 0, 0" "0.750000,0.750000,0.750000") "Undefined" 0 0)
        (Math|Integer|IncrementInt (Variables|Default|GetH2O2%20Count))))
    (:then_3
      (if (not (>= (Variables|Default|GetCO2%20Count) (Math|Random|RandomIntegerinRange 10 15)))
        (Game|SpawnActorfromClass "/Game/Blueprints/CO2.CO2_C" (Math|Transform|MakeTransform _returnvalue_2 "0, 0, 0" "0.750000,0.750000,0.750000") "Undefined" 0 0)
        (Math|Integer|IncrementInt (Variables|Default|GetCO2%20Count))))
    (:then_4
      (if (not (>= (Variables|Default|GetNH3%20Count) (Math|Random|RandomIntegerinRange 10 15)))
        (Game|SpawnActorfromClass "/Game/Blueprints/NH3.NH3_C" (Math|Transform|MakeTransform _returnvalue_2 "0, 0, 0" "0.750000,0.750000,0.750000") "Undefined" 0 0)
        (Math|Integer|IncrementInt (Variables|Default|GetNH3%20Count))))))

(fn ConstructionScript)